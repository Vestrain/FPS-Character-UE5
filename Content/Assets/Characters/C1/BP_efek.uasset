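; Player character Blueprint that handles Enhanced Input walking, looking, jumping and crouching.
; Crouching blocks jumping, lowers walk speed and uses a Timeline to smoothly shrink the capsule's half height.
; Releasing crouch restores both only when a capsule trace macro finds no overhead obstruction.
; Tick repeats that trace and, after detecting an obstruction, rechecks following a short Delay to stand the character up once clear.
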(event EventBeginPlay
  ;[1 1 1] Enhanced Input Setup
  (bind _asplayer_controller (Utilities|Casting|CastToPlayerController (Pawn|GetController)))
  (Utilities|IsValid (PlayerController|LocalPlayerSubsystems|GetEnhancedInputLocalPlayerSubsystem _asplayer_controller)
    (:Is%20Valid
      (Input|AddMappingContext (PlayerController|LocalPlayerSubsystems|GetEnhancedInputLocalPlayerSubsystem _asplayer_controller) "/Game/Inputs/IMC_Default.IMC_Default" 0 "(bIgnoreAllPressedKeysUntilRelease=True,bForceImmediately=False)")
      (Variables|Default|SetMax%20Walk%20Speed (Variables|/Script/Engine.CharacterMovementComponent|GetMaxWalkSpeed (Variables|Character|GetCharacterMovement)))
      (Variables|Default|SetCapsule%20Half%20Height (Variables|/Script/Engine.CapsuleComponent|GetCapsuleHalfHeight (Variables|Collision|GetCapsuleComponent))))))

(event EventTick
  (params (DeltaSeconds :type Float%20%28single-precision%29))
  (CallFunction|Uncrouchthingy))

(event Custom|uncrouchthingy
  ;[1 1 1] Crouch
  (Utilities|CheckRoofMacro
    (:true
      (Utilities|FlowControl|Delay 0.1)
      (Utilities|CheckRoofMacro
        (:else
          (Variables|Default|SetSomethingOnTop false)
          (Variables|/Script/Engine.CharacterMovementComponent|SetMaxWalkSpeed (Variables|Character|GetCharacterMovement) (Variables|Default|GetMax%20Walk%20Speed))
          (Variables|Default|SetCrouched false)
          (bind _crouch (Timeline|Timeline Reverse)
            (:Update
              (Components|Capsule|SetCapsuleHalfHeight (Variables|Collision|GetCapsuleComponent) (Math|Float|Lerp (Variables|Default|GetCapsule%20Half%20Height) 3e+01 _crouch) true))))))))

(event Input|EnhancedActionEvents|EnhancedInputActionMoveForward
  (params (ActionValue :type Float%20%28double-precision%29) (ElapsedSeconds :type Float%20%28double-precision%29) (TriggeredSeconds :type Float%20%28double-precision%29) (InputAction :type Input%20Action%20Object%20Reference :default "/Game/Inputs/Actions/MoveForward.MoveForward"))
  ;[1 1 1] Movement
  (:Triggered
    (Pawn|Input|AddMovementInput (Math|Vector|GetForwardVector (Math|Rotator|MakeRotator 0.0 0.0 (.Yaw (Math|Rotator|BreakRotator (Pawn|GetControlRotation :!class /Script/Engine.Pawn))))) ActionValue false)))

(event Input|EnhancedActionEvents|EnhancedInputActionMoveRight
  (params (ActionValue :type Float%20%28double-precision%29) (ElapsedSeconds :type Float%20%28double-precision%29) (TriggeredSeconds :type Float%20%28double-precision%29) (InputAction :type Input%20Action%20Object%20Reference :default "/Game/Inputs/Actions/MoveRight.MoveRight"))
  ;[1 1 1] Movement
  (:Triggered
    (Pawn|Input|AddMovementInput (Math|Vector|GetRightVector (Math|Rotator|MakeRotator 0.0 0.0 (.Yaw (Math|Rotator|BreakRotator (Pawn|GetControlRotation :!class /Script/Engine.Pawn))))) ActionValue false)))

(event Input|EnhancedActionEvents|EnhancedInputActionJump
  (params (ActionValue :type Boolean) (ElapsedSeconds :type Float%20%28double-precision%29) (TriggeredSeconds :type Float%20%28double-precision%29) (InputAction :type Input%20Action%20Object%20Reference :default "/Game/Inputs/Actions/Jump.Jump"))
  ;[1 1 1] Jump & Crouch
  (:Triggered
    (if (not (Variables|Default|GetCrouched))
      (Character|Jump)))
  (:Canceled
    (Character|StopJumping)))

(event Input|EnhancedActionEvents|EnhancedInputActionCrouch
  (params (ActionValue :type Boolean) (ElapsedSeconds :type Float%20%28double-precision%29) (TriggeredSeconds :type Float%20%28double-precision%29) (InputAction :type Input%20Action%20Object%20Reference :default "/Game/Inputs/Actions/Crouch.Crouch"))
  (bind _charactermovement (Variables|Character|GetCharacterMovement))
  ;[1 1 1] Crouch
  (:Triggered
    (if ActionValue
      (Variables|/Script/Engine.CharacterMovementComponent|SetMaxWalkSpeed _charactermovement (Variables|/Script/Engine.CharacterMovementComponent|GetMaxWalkSpeedCrouched _charactermovement))
      (Variables|Default|SetCrouched true)
      (bind _crouch (Timeline|Timeline Play)
        (:Update
          (Components|Capsule|SetCapsuleHalfHeight (Variables|Collision|GetCapsuleComponent) (Math|Float|Lerp (Variables|Default|GetCapsule%20Half%20Height) 3e+01 _crouch) true)))
      (else
        (Utilities|CheckRoofMacro
          (:else
            (Variables|Default|SetSomethingOnTop false)
            (Variables|/Script/Engine.CharacterMovementComponent|SetMaxWalkSpeed _charactermovement (Variables|Default|GetMax%20Walk%20Speed))
            (Variables|Default|SetCrouched false)
            (Timeline|Timeline Reverse))
          (:true
            (Variables|Default|SetSomethingOnTop true)))))))

(event Input|EnhancedActionEvents|EnhancedInputActionLookUp
  (params (ActionValue :type Float%20%28double-precision%29) (ElapsedSeconds :type Float%20%28double-precision%29) (TriggeredSeconds :type Float%20%28double-precision%29) (InputAction :type Input%20Action%20Object%20Reference :default "/Game/Inputs/Actions/LookUp.LookUp"))
  (:Triggered
    (Pawn|Input|AddControllerPitchInput ActionValue)))

(event Input|EnhancedActionEvents|EnhancedInputActionLookRight
  (params (ActionValue :type Float%20%28double-precision%29) (ElapsedSeconds :type Float%20%28double-precision%29) (TriggeredSeconds :type Float%20%28double-precision%29) (InputAction :type Input%20Action%20Object%20Reference :default "/Game/Inputs/Actions/LookRight.LookRight"))
  (:Triggered
    (Pawn|Input|AddControllerYawInput ActionValue)))

(fn ConstructionScript)